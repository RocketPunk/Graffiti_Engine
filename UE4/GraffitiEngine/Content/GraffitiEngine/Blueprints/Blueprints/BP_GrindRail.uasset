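; BP_GrindRail is a spline-based grind rail that converts a world location into a distance along its spline.
; GetDistanceAtLocationAlongSpline finds the closest input key, then linearly interpolates between the distances of the surrounding spline points using the key's fractional part.
; The construction script only calls its parent, and the grinding movement itself is not handled in these graphs.
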(fn `GetDistanceAtLocationAlongSpline`
  (params (Location :type "Vector Structure"))
  (returns (Distance :type "Float (double-precision)"))
  (bind _spline (`self.Spline`))
  (bind _returnvalue (`SplineComponent.FindInputKeyClosestToWorldLocation` _spline Location))
  (bind _returnvalue_2 (`KismetMathLibrary.FTrunc` _returnvalue))
  (bind _returnvalue_3 (`SplineComponent.GetDistanceAlongSplineAtSplinePoint` _spline _returnvalue_2))
  (return (+ _returnvalue_3 (* (- (`SplineComponent.GetDistanceAlongSplineAtSplinePoint` _spline (`KismetMathLibrary.FTrunc` (+ _returnvalue 1.0))) _returnvalue_3) (- _returnvalue (`KismetMathLibrary.Conv_IntToDouble` _returnvalue_2))))))

(fn `UserConstructionScript`
  (`parent.UserConstructionScript`))