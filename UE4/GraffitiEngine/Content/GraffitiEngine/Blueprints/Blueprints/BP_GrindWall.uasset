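; BP_GrindWall is a spline-built wall the player can grind along at the height where contact is made.
; Construction lays spline meshes with a grind signifier material along VisualSpline, and BeginPlay copies its points and tangents into GrindSpline.
; PlayerContact moves GrindSpline to the contact Z and disables wall collision, which EndGrind re-enables.
; Helpers interpolate distance along VisualSpline from a location and return GrindSpline's right vector as the off-wall direction.
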(event `self.ReceiveBeginPlay`
  (bind _visualspline (`self.VisualSpline`))
  (bind _grindspline (`self.GrindSpline`))
  (for _index (range (`SplineComponent.GetNumberOfSplinePoints` (`self.VisualSpline`)))
    (`SplineComponent.AddSplinePoint` _grindspline (`SplineComponent.GetLocationAtSplinePoint` _visualspline _index "Local") "Local" true)
    (`SplineComponent.SetTangentsAtSplinePoint` _grindspline _index (`SplineComponent.GetArriveTangentAtSplinePoint` _visualspline _index "Local") (`SplineComponent.GetLeaveTangentAtSplinePoint` _visualspline _index "Local") "Local" true)))

(event `ToggleWallCollision`
  (params (ColiisionEnabled :type Boolean))
  (for _array_element (`self.K2_GetComponentsByClass` "/Script/Engine.SplineMeshComponent")
    (if ColiisionEnabled
      (`PrimitiveComponent.SetCollisionEnabled` _array_element "QueryAndPhysics")
      (else
        (`PrimitiveComponent.SetCollisionEnabled` _array_element "NoCollision")))))

(event `PlayerContact`
  (params (ContactLocation :type "Vector Structure"))
  (bind _grindspline (`self.GrindSpline`))
  (bind (_returnvalue_x _returnvalue_y) (`KismetMathLibrary.BreakVector` (`SceneComponent.K2_GetComponentLocation` _grindspline)))
  (`SceneComponent.K2_SetWorldLocation` _grindspline (`KismetMathLibrary.MakeVector` _returnvalue_x _returnvalue_y (.z ContactLocation)) false false)
  (`self.ToggleWallCollision` false))

(event `EndGrind`
  (`self.ToggleWallCollision` true))

(fn `GetDistanceAtLocationAlongSpline`
  (params (Location :type "Vector Structure"))
  (returns (Distance :type "Float (double-precision)"))
  (bind _visualspline (`self.VisualSpline`))
  (bind _returnvalue (`SplineComponent.FindInputKeyClosestToWorldLocation` _visualspline Location))
  (bind _returnvalue_2 (`KismetMathLibrary.FTrunc` _returnvalue))
  (bind _returnvalue_3 (`SplineComponent.GetDistanceAlongSplineAtSplinePoint` _visualspline _returnvalue_2))
  (return (+ _returnvalue_3 (* (- (`SplineComponent.GetDistanceAlongSplineAtSplinePoint` _visualspline (`KismetMathLibrary.FTrunc` (+ _returnvalue 1.0))) _returnvalue_3) (- _returnvalue (`KismetMathLibrary.Conv_IntToDouble` _returnvalue_2))))))

(fn `GetOffWallVector`
  (params (Distance :type "Float (double-precision)"))
  (returns (OffWallVector :type "Vector Structure"))
  (return (`SplineComponent.GetRightVectorAtDistanceAlongSpline` (`self.GrindSpline`) Distance "World")))

(fn `UserConstructionScript`
  (bind _visualspline (`self.VisualSpline`))
  (`|ExecutionSequence`
    (:`then_0`
      (`SplineComponent.ClearSplinePoints` (`self.GrindSpline`) true))
    (:`then_1`
      (for _index (range (+ (- (`SplineComponent.GetNumberOfSplinePoints` _visualspline) 2) 1))
        (bind _returnvalue (`AddComponent|NODE_AddSplineMeshComponent-0`))
        (`PrimitiveComponent.SetMaterial` _returnvalue 0 "/Game/Materials/M_WallGrindSignifier.M_WallGrindSignifier")
        (`PrimitiveComponent.SetCollisionObjectType` _returnvalue "ECC_GameTraceChannel1")
        (`StaticMeshComponent.SetStaticMesh` _returnvalue (`self.Mesh`))
        (`SplineMeshComponent.SetForwardAxis` _returnvalue (`self.ForwardAxis`) true)
        (`self.K2_AttachToComponent` _visualspline "None" "KeepRelative" "KeepRelative" "KeepRelative")
        (bind _returnvalue_2 (+ _index 1))
        (`SplineMeshComponent.SetStartAndEnd` _returnvalue (`SplineComponent.GetLocationAtSplinePoint` _visualspline _index "Local") (`SplineComponent.GetTangentAtSplinePoint` _visualspline _index "Local") (`SplineComponent.GetLocationAtSplinePoint` _visualspline _returnvalue_2 "Local") (`SplineComponent.GetTangentAtSplinePoint` _visualspline _returnvalue_2 "Local") true)
        (`PrimitiveComponent.SetCollisionEnabled` _returnvalue "QueryOnly")))))