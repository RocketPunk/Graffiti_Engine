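; BP_DestructableObject is a prop that shatters when a rollerskater pawn hits it fast enough, then fades away.
; Construction applies the chosen destructible mesh, a dynamic signifier material and the detection bounds.
; Overlap above the breaking threshold enables physics and applies damage along the skater's surface detector forward, with impulse scaled by velocity.
; A timer based on debris lifetime then fades material opacity through a timeline and destroys the actor.
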(event `self.ReceiveBeginPlay`
  (`PrimitiveComponent.SetSimulatePhysics` (`self.DestructableMesh`) (`self.StartWithPhysics`)))

(event `self.CollisionDetection.OnComponentBeginOverlap`
  (params (OverlappedComponent :type "PrimitiveComponent Object Reference") (OtherActor :type "Actor Object Reference") (OtherComp :type "PrimitiveComponent Object Reference") (OtherBodyIndex :type Integer) (bFromSweep :type Boolean) (SweepResult :type "HitResult Structure (by ref)"))
  (bind _destructablemesh (`self.DestructableMesh`))
  (bind _aspawn_rollerskater (cast `/Game/Blueprints/Pawn_Rollerskater` OtherActor))
  (bind _output_get (set `self.Pawn` _aspawn_rollerskater))
  (bind _velocity (`/Game/Blueprints/Pawn_Rollerskater.Velocity` _output_get))
  (if (>= _velocity (`self.BreakingThreshold`))
    (`PrimitiveComponent.SetSimulatePhysics` _destructablemesh true)
    (bind _surfacedetector (`/Game/Blueprints/Pawn_Rollerskater.SurfaceDetector` _output_get))
    (`DestructibleComponent.ApplyDamage` _destructablemesh 1000.0 (`SceneComponent.K2_GetComponentLocation` _surfacedetector) (`SceneComponent.GetForwardVector` _surfacedetector) (* (* _velocity 250.0) (`self.FractureMultiplier`)))
    (`KismetSystemLibrary.K2_SetTimerDelegate` (delegate `Death`) (- (`self.DebrisLifetime`) 1.0))))

(event `Death`
  (bind (_direction _opacity) (`Timeline|Fade` :!via `PlayFromStart`)
    (:`Update`
      (`MaterialInstanceDynamic.SetScalarParameterValue` (`self.Material`) "Opacity" _opacity))
    (:`Finished`
      (`self.K2_DestroyActor`))))

(fn `UserConstructionScript`
  (bind _destructablemesh (`self.DestructableMesh`))
  (`DestructibleComponent.SetDestructibleMesh` _destructablemesh (`self.DestructableMeshOverride`))
  (bind _returnvalue (`KismetMaterialLibrary.CreateDynamicMaterialInstance` "/Game/Materials/M_DestructableSignifier.M_DestructableSignifier"))
  (bind _output_get (set `self.Material` _returnvalue))
  (`PrimitiveComponent.SetMaterial` _destructablemesh 0 _output_get)
  (`SceneComponent.SetRelativeScale3D` (`self.CollisionDetection`) (`self.DetectionBounds`)))